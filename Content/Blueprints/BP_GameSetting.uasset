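; BP_GameSetting sets up a Crewmate-versus-Impostor match on BeginPlay, spawning both roles and giving the first player control of one.
; SpawnPlayers shuffles all PlayerStarts, then spawns the configured crewmate count followed by impostors at the next indices, skipping any beyond the available starts.
; CharacterType, resolved by coin flip when set to Random, is printed in a role color and picks which class player 0 possesses, choosing a random instance.
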(event EventBeginPlay
  (Utilities|FlowControl|Sequence
    (:then_0
      (CallFunction|SpawnPlayers))
    (:then_1
      (Utilities|FlowControl|Sequence
        (:then_0
          (if (Utilities|Enum|Equal(Enum) (Variables|Default|GetcharacterType) "NewEnumerator3")
            (Variables|Default|SetcharacterType (select (Math|Random|RandomBool) "NewEnumerator2" "NewEnumerator1"))))
        (:then_1
          (Development|PrintString (Utilities|String|EnumtoString (Variables|Default|GetcharacterType)) true true (Utilities|Select :Index (Variables|Default|GetcharacterType) :NewEnumerator0 "" :NewEnumerator1 "(R=0.187233,G=1.000000,B=0.980103,A=1.000000)" :NewEnumerator2 "(R=0.473958,G=0.000000,B=0.000000,A=1.000000)" :NewEnumerator3 ""))
          (switch Utilities|FlowControl|Switch|Switchone_CharacterType (Variables|Default|GetcharacterType)
            (:NewEnumerator1
              (bind _outactors (Actor|GetAllActorsOfClass "/Game/ThirdPersonBP/Blueprints/BP_Crewmate.BP_Crewmate_C"))
              (Pawn|Possess (Game|GetPlayerController 0) (Utilities|Array|Get(acopy) _outactors (Math|Random|RandomInteger (Utilities|Array|Length _outactors)))))
            (:NewEnumerator2
              (bind _outactors_2 (Actor|GetAllActorsOfClass "/Game/ThirdPersonBP/Blueprints/BP_Impostor.BP_Impostor_C"))
              (Pawn|Possess (Game|GetPlayerController 0) (Utilities|Array|Get(acopy) _outactors_2 (Math|Random|RandomInteger (Utilities|Array|Length _outactors_2)))))))))))

(fn ConstructionScript)

(fn SpawnPlayers
  (Utilities|FlowControl|Sequence
    (:then_0
      (bind _outactors (Actor|GetAllActorsOfClass "/Script/Engine.PlayerStart"))
      (LocalVariables|SetplayerStarts_l _outactors)
      (Utilities|Array|Shuffle (LocalVariables|GetplayerStarts_l)))
    (:then_1
      (Utilities|FlowControl|Sequence
        (:then_0
          (for _index (range 0 (- (Variables|Default|GetcrewmateCount) 1))
            (if (Utilities|Array|IsValidIndex (LocalVariables|GetplayerStarts_l) _index)
              (Game|SpawnActorfromClass "/Game/ThirdPersonBP/Blueprints/BP_Crewmate.BP_Crewmate_C" (Math|Transform|MakeTransform (Transformation|GetActorLocation (Utilities|Array|Get(acopy) (LocalVariables|GetplayerStarts_l) _index)) (Transformation|GetActorRotation (Utilities|Array|Get(acopy) (LocalVariables|GetplayerStarts_l) _index))) "Undefined" 0 0))))
        (:then_1
          (for _index_2 (range 0 (- (Variables|Default|GetimpostorCount) 1))
            (if (Utilities|Array|IsValidIndex (LocalVariables|GetplayerStarts_l) (+ (Variables|Default|GetcrewmateCount) _index_2))
              (Game|SpawnActorfromClass "/Game/ThirdPersonBP/Blueprints/BP_Impostor.BP_Impostor_C" (Math|Transform|MakeTransform (Transformation|GetActorLocation (Utilities|Array|Get(acopy) (LocalVariables|GetplayerStarts_l) (+ (Variables|Default|GetcrewmateCount) _index_2))) (Transformation|GetActorRotation (Utilities|Array|Get(acopy) (LocalVariables|GetplayerStarts_l) (+ (Variables|Default|GetcrewmateCount) _index_2)))) "Undefined" 0 0))))))))