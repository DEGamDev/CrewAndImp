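; Vent actor that swings open by pitching its RotateRoot component up to a right angle.
; The Open event plays a timeline from the start, interpolating the pitch with its alpha, and BeginPlay raises the timeline's play rate for a quick motion.
; A helper function returns the look-at yaw from this actor to another given vent.
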(event Custom|Open
  (bind _alpha (Timeline|TL_Open PlayFromStart)
    (:Update
      (Transformation|SetRelativeRotation (Variables|Default|GetRotateRoot) (Math|Rotator|MakeRotator 0.0 (Math|Float|Lerp 0.0 9e+01 _alpha) 0.0) false false))))

(event EventBeginPlay
  (Components|Timeline|SetPlayRate (Variables|Default|GetTL_Open) 5.0))

(event Collision|EventActorBeginOverlap
  (params (OtherActor :type Actor%20Object%20Reference)))

(event EventTick
  (params (DeltaSeconds :type Float%20%28single-precision%29)))

(fn ConstructionScript)

(fn GetTargetAngle
  (params (vent :type BP%20Vent%20Object%20Reference))
  (return (.Yaw (Math|Rotator|BreakRotator (Math|Rotator|FindLookatRotation (Transformation|GetActorLocation) (Transformation|GetActorLocation vent))))))