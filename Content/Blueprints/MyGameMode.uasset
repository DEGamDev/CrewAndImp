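; MyGameMode is a game mode that tracks task completion and assigns each character a color and number.
; On BeginPlay it counts the BP_Task actors in the level, then gathers every BP_Character, coloring each from AllColors by array index and storing that index as its Number.
; CompletedTaskPercent returns CompletedTaskCount over the total task count as a 0–1 fraction; nothing in this file updates the completed count.
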(event EventBeginPlay
  (Utilities|FlowControl|Sequence
    (:then_0
      (bind _outactors (Actor|GetAllActorsOfClass "/Game/Blueprints/BP_Task.BP_Task_C"))
      (Variables|Default|SetallTaskCount (Utilities|Array|Length _outactors)))
    (:then_1
      (Utilities|FlowControl|Sequence
        (:then_0
          (bind _outactors_2 (Actor|GetAllActorsOfClass "/Game/ThirdPersonBP/Blueprints/BP_Character.BP_Character_C"))
          (Variables|Default|SetallCharacter _outactors_2))
        (:then_1
          (for (_array_element _array_index) (Variables|Default|GetallCharacter)
            (Default|SetColor _array_element (Utilities|Array|Get(acopy) (Variables|Default|GetallColors) _array_index))
            (Variables|/Game/ThirdPersonBP/Blueprints/BP_Character.BP_Character_C|Setnumber _array_element _array_index)))))))

(event EventTick
  (params (DeltaSeconds :type Float%20%28single-precision%29)))

(fn ConstructionScript)

(fn CompletedTaskPercent
  (return (/ (Math|Conversions|ToFloat(Integer) (Variables|Default|GetcompletedTaskCount)) (Math|Conversions|ToFloat(Integer) (Variables|Default|GetallTaskCount)))))